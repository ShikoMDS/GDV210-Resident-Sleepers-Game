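; BP_Switch_A is an interactable switch that changes two lights and completes the first UI objective.
; On BeginPlay it spawns two BP_BasicLight actors at local LightPos offsets converted to world space, then moves each Bulb to its actor's location.
; Interact swaps the material on both bulbs, then finds all BPW_UI widgets and calls CompleteObj1 on them.
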(event EventBeginPlay
  (bind _returnvalue (Game|SpawnActorfromClass "/Game/Blueprints/BP_BasicLight.BP_BasicLight_C" (Math|Conversions|ToTransform(Vector) (Math|Transform|TransformLocation (Transformation|GetWorldTransform (Variables|Default|GetDefaultSceneRoot)) (Variables|Default|GetLightPos1))) "Undefined" "MultiplyWithRoot" 0 0))
  (bind _output_get (Variables|Default|SetLight1 _returnvalue))
  (Transformation|SetWorldLocation (Variables|/Game/Blueprints/BP_BasicLight.BP_BasicLight_C|GetBulb _output_get) (Transformation|GetActorLocation _output_get) false false)
  (bind _returnvalue_2 (Game|SpawnActorfromClass "/Game/Blueprints/BP_BasicLight.BP_BasicLight_C" (Math|Conversions|ToTransform(Vector) (Math|Transform|TransformLocation (Transformation|GetWorldTransform (Variables|Default|GetDefaultSceneRoot)) (Variables|Default|GetLightPos2))) "Undefined" "MultiplyWithRoot" 0 0))
  (bind _output_get_2 (Variables|Default|SetLight2 _returnvalue_2))
  (Transformation|SetWorldLocation (Variables|/Game/Blueprints/BP_BasicLight.BP_BasicLight_C|GetBulb _output_get_2) (Transformation|GetActorLocation _output_get_2) false false))

(event Collision|EventActorBeginOverlap
  (params (OtherActor :type Actor%20Object%20Reference)))

(event EventTick
  (params (DeltaSeconds :type Float%20%28single-precision%29)))

(event EventInteract
  (Rendering|Material|SetMaterial (Variables|/Game/Blueprints/BP_BasicLight.BP_BasicLight_C|GetBulb (Variables|Default|GetLight1)) 0 "/Game/ReubenAssets/standardSurface2.standardSurface2")
  (bind _foundwidgets (Widget|GetAllWidgetsOfClass "/Game/UI/BPW_UI.BPW_UI_C" false))
  (Default|CompleteObj1 _foundwidgets))

(fn ConstructionScript)
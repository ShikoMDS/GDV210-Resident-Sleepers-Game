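; BP_Transformer is an interactable transformer that switches off the street lamps and completes the fourth objective.
; On its first Interact, it sets a Completed flag, plays a switch sound and loops over every BP_StreetLamp, zeroing its spotlight and swapping a mesh material.
; Inside that loop it also looks up BPW_UI widgets and calls CompleteObj4, so the objective call repeats for each lamp.
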(event EventBeginPlay)

(event Collision|EventActorBeginOverlap
  (params (OtherActor :type Actor%20Object%20Reference)))

(event EventTick
  (params (DeltaSeconds :type Float%20%28single-precision%29)))

(event EventInteract
  (if (not (Variables|Default|Getcompleted))
    (Variables|Default|Setcompleted true)
    (Audio|PlaySound2D "/Game/Movies/switch3.switch3" 1.0 1.0 0.0 0 0)
    (bind _outactors (Actor|GetAllActorsOfClass "/Game/Blueprints/BP_StreetLamp.BP_StreetLamp_C"))
    (for _array_element _outactors
      (Rendering|Components|Light|SetIntensity (Variables|/Game/Blueprints/BP_StreetLamp.BP_StreetLamp_C|GetSpotLight _array_element) 0.0)
      (Rendering|Material|SetMaterial (Variables|/Game/Blueprints/BP_StreetLamp.BP_StreetLamp_C|GetStaticMesh _array_element) 1 "/Game/ReubenAssets/standardSurface2.standardSurface2")
      (bind _foundwidgets (Widget|GetAllWidgetsOfClass "/Game/UI/BPW_UI.BPW_UI_C" false))
      (Default|CompleteObj4 _foundwidgets))))

(fn ConstructionScript)
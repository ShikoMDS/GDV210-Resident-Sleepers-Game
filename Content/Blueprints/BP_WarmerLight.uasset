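; BP_WarmerLight is an interactable ceiling light that switches to a warm tint and completes the fifth objective in the UI.
; On Interact, it swaps the bulb to the dim ceiling-light material, then sets a fixed intensity and warm color on its point and spot lights.
; It then finds BPW_UI widgets by class and calls CompleteObj5 on them, with no guard against repeat interactions.
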(event EventBeginPlay)

(event Collision|EventActorBeginOverlap
  (params (OtherActor :type Actor%20Object%20Reference)))

(event EventTick
  (params (DeltaSeconds :type Float%20%28single-precision%29)))

(event EventInteract
  (Rendering|Material|SetMaterial (Variables|Default|GetBulb) 0 "/Game/Materials/InstancedMaterials/INST_CeilingLightDim.INST_CeilingLightDim")
  (Rendering|Components|Light|SetIntensity (Variables|Default|GetPointLight) 1e+04)
  (Rendering|Components|Light|SetLightColor (Variables|Default|GetPointLight) "(R=0.162029,G=0.099899,B=0.004025,A=1.000000)" true)
  (Rendering|Components|Light|SetLightColor (Variables|Default|GetSpotLight) "(R=0.162029,G=0.099899,B=0.004025,A=1.000000)" true)
  (Rendering|Components|Light|SetIntensity (Variables|Default|GetSpotLight) 1e+04)
  (bind _foundwidgets (Widget|GetAllWidgetsOfClass "/Game/UI/BPW_UI.BPW_UI_C" false))
  (Default|CompleteObj5 _foundwidgets))

(fn ConstructionScript)
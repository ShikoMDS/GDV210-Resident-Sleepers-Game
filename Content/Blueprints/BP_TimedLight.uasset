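; BP_TimedLight is a proximity-driven pair of spotlights that the player first enables through Interact.
; The first Interact sets IsOn, plays a switch sound and calls CompleteObj8 on BPW_UI.
; Once enabled, the first-person character entering Range lights both bulbs by swapping materials and raising intensity.
; Leaving Range darkens them after a short delay, which re-entry does not cancel.
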(event OnComponentBeginOverlap(range)
  (params (OverlappedComponent :type Primitive%20Component%20Object%20Reference) (OtherActor :type Actor%20Object%20Reference) (OtherComp :type Primitive%20Component%20Object%20Reference) (OtherBodyIndex :type Integer) (bFromSweep :type Boolean) (SweepResult :type Hit%20Result%20Structure%20%28by%20ref%29))
  (Utilities|Casting|CastToBP_FirstPersonCharacter OtherActor)
  (if (Variables|Default|Getis_on)
    (Rendering|Material|SetMaterial (Variables|Default|Getbulb1) 0 "/Game/Materials/InstancedMaterials/INST_CeilingLight.INST_CeilingLight")
    (Rendering|Components|Light|SetIntensity (Variables|Default|GetSpotLightA) 5e+03)
    (Rendering|Material|SetMaterial (Variables|Default|Getbulb2) 0 "/Game/Materials/InstancedMaterials/INST_CeilingLight.INST_CeilingLight")
    (Rendering|Components|Light|SetIntensity (Variables|Default|GetSpotLightB) 5e+03)))

(event OnComponentEndOverlap(range)
  (params (OverlappedComponent :type Primitive%20Component%20Object%20Reference) (OtherActor :type Actor%20Object%20Reference) (OtherComp :type Primitive%20Component%20Object%20Reference) (OtherBodyIndex :type Integer))
  (Utilities|Casting|CastToBP_FirstPersonCharacter OtherActor)
  (if (Variables|Default|Getis_on)
    (Utilities|FlowControl|Delay 2.0)
    (Rendering|Material|SetMaterial (Variables|Default|Getbulb1) 0 "/Game/ReubenAssets/standardSurface2.standardSurface2")
    (Rendering|Components|Light|SetIntensity (Variables|Default|GetSpotLightA) 0.0)
    (Rendering|Material|SetMaterial (Variables|Default|Getbulb2) 0 "/Game/ReubenAssets/standardSurface2.standardSurface2")
    (Rendering|Components|Light|SetIntensity (Variables|Default|GetSpotLightB) 0.0)))

(event EventBeginPlay)

(event Collision|EventActorBeginOverlap
  (params (OtherActor :type Actor%20Object%20Reference)))

(event EventTick
  (params (DeltaSeconds :type Float%20%28single-precision%29)))

(event EventInteract
  (if (not (Variables|Default|Getis_on))
    (Variables|Default|Setis_on true)
    (Audio|PlaySound2D "/Game/Movies/switch3.switch3" 1.0 1.0 0.0 0 0)
    (bind _foundwidgets (Widget|GetAllWidgetsOfClass "/Game/UI/BPW_UI.BPW_UI_C" false))
    (Default|CompleteObj8 _foundwidgets)))

(fn ConstructionScript)
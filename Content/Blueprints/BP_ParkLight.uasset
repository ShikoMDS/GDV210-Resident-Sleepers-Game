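; BP_ParkLight is an interactable park light that serves as objective 6 and can be switched off once.
; Its Interact event plays a switch sound, swaps a mesh material and sets the spotlight intensity to zero, guarded by a Completed flag.
; It then marks the objective complete on the BPW_UI widgets and in BP_GameInstance, which checks whether all objectives are done.
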(event EventBeginPlay)

(event Collision|EventActorBeginOverlap
  (params (OtherActor :type Actor%20Object%20Reference)))

(event EventTick
  (params (DeltaSeconds :type Float%20%28single-precision%29)))

(event EventInteract
  (if (not (Variables|Default|Getcompleted))
    (Variables|Default|Setcompleted true)
    (Audio|PlaySound2D "/Game/SFX-Music/switch3.switch3" 1.0 1.0 0.0 0 0)
    (Rendering|Material|SetMaterial (Variables|Default|GetStaticMesh1) 1 "/Game/ReubenAssets/standardSurface2.standardSurface2")
    (Rendering|Components|Light|SetIntensity (Variables|Default|GetSpotLight) 0.0)
    (bind _foundwidgets (Widget|GetAllWidgetsOfClass "/Game/UI/BPW_UI.BPW_UI_C" false))
    (Default|CompleteObj6 _foundwidgets)
    (bind _asbp_game_instance (Utilities|Casting|CastToBP_GameInstance (Game|GetGameInstance)))
    (Variables|/Game/Blueprints/BP_GameInstance.BP_GameInstance_C|SetObj6 _asbp_game_instance true)
    (Default|CheckAllCompleteEvent _asbp_game_instance)))

(fn ConstructionScript)
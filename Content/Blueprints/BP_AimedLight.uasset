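; BP_AimedLight is an interactable pair of lamps that can be re-aimed once and completes objective 7.
; On the first Interact it plays a switch sound, snaps both lamps to fixed rotations and calls CompleteObj7 on the BPW_UI widgets it finds.
; After a short delay it swaps both bulb materials and sets both spotlights to zero intensity, switching the lights off.
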(event EventBeginPlay)

(event Collision|EventActorBeginOverlap
  (params (OtherActor :type Actor%20Object%20Reference)))

(event EventTick
  (params (DeltaSeconds :type Float%20%28single-precision%29)))

(event EventInteract
  (if (not (Variables|Default|Getis_moved))
    (Audio|PlaySound2D "/Game/Movies/switch3.switch3" 1.0 1.0 0.0 0 0)
    (Variables|Default|Setis_moved true)
    (Transformation|SetRelativeRotation (Variables|Default|Getlamp1) "50.000000,130.000000,-180.000000" false false)
    (Transformation|SetRelativeRotation (Variables|Default|Getlamp2) "-50.000000,-130.000000,-180.000000" false false)
    (bind _foundwidgets (Widget|GetAllWidgetsOfClass "/Game/UI/BPW_UI.BPW_UI_C" false))
    (Default|CompleteObj7 _foundwidgets)
    (Utilities|FlowControl|Delay 2.0)
    (Rendering|Material|SetMaterial (Variables|Default|Getbulb1) 0 "/Game/ReubenAssets/standardSurface2.standardSurface2")
    (Rendering|Components|Light|SetIntensity (Variables|Default|GetSpotLightA) 0.0)
    (Rendering|Material|SetMaterial (Variables|Default|Getbulb2) 0 "/Game/ReubenAssets/standardSurface2.standardSurface2")))

(fn ConstructionScript)